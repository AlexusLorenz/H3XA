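; Actor component that tracks the current score and persists a name-to-score highscore table in a save game.
; AddPoints and ResetPoints update Score and broadcast it through OnScoreChanged.
; SaveToHighscores writes Score into the SG_Highscrores slot; when creating a new save, it uses the literal "Name" instead of the passed name.
; LoadHighscores returns the saved table, creating and saving an empty one if none exists.
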(event `AddPoints`
  (params (Points :type Integer))
  (bind _output_get (set `self.Score` (+ (stale _output_get) Points)))
  (`self.onScoreChanged` _output_get))

(event `ResetPoints`
  (bind _output_get (set `self.Score` 0))
  (`self.onScoreChanged` _output_get))

(fn `LoadHighscores`
  (returns (Highscores :type "Map of Name to Integer"))
  (locals (_CurrentSavegame :type "SaveGame Object Reference"))
  (bind _returnvalue (`GameplayStatics.DoesSaveGameExist` (`self.SaveSlot`)))
  (if _returnvalue
    (bind _returnvalue_2 (`GameplayStatics.LoadGameFromSlot` (`self.SaveSlot`)))
    (bind _output_get (set `local._CurrentSavegame` _returnvalue_2))
    (bind _assg_highscrores (cast `/Game/02_Modules/HighscoreSystem/SG_Highscrores` _output_get))
    (return (`/Game/02_Modules/HighscoreSystem/SG_Highscrores.Highscores` _assg_highscrores))
    (else
      (bind _returnvalue_3 (`GameplayStatics.CreateSaveGameObject` "/Game/02_Modules/HighscoreSystem/SG_Highscrores.SG_Highscrores_C"))
      (`GameplayStatics.SaveGameToSlot` _returnvalue_3 (`self.SaveSlot`))
      (return (`/Game/02_Modules/HighscoreSystem/SG_Highscrores.Highscores` _returnvalue_3)))))

(fn `SaveToHighscores`
  (params (Name :type Name))
  (locals (Highscores :type "Map of Name to Integer") (_CurrentSavegame :type "SaveGame Object Reference"))
  (bind _returnvalue (`GameplayStatics.DoesSaveGameExist` (`self.SaveSlot`)))
  (if _returnvalue
    (bind _returnvalue_2 (`GameplayStatics.LoadGameFromSlot` (`self.SaveSlot`)))
    (bind _output_get (set `local._CurrentSavegame` _returnvalue_2))
    (bind _assg_highscrores (cast `/Game/02_Modules/HighscoreSystem/SG_Highscrores` _output_get))
    (bind _highscores (`/Game/02_Modules/HighscoreSystem/SG_Highscrores.Highscores` _assg_highscrores))
    (set `self.Highscores` _highscores)
    (`BlueprintMapLibrary.Map_Add` _highscores (`local.Name`) (`self.Score`))
    (`GameplayStatics.SaveGameToSlot` (`local._CurrentSavegame`) (`self.SaveSlot`))
    (else
      (bind _returnvalue_3 (`GameplayStatics.CreateSaveGameObject` "/Game/02_Modules/HighscoreSystem/SG_Highscrores.SG_Highscrores_C"))
      (`BlueprintMapLibrary.Map_Add` (`/Game/02_Modules/HighscoreSystem/SG_Highscrores.Highscores` _returnvalue_3) "Name" (`self.Score`))
      (`GameplayStatics.SaveGameToSlot` _returnvalue_3 (`self.SaveSlot`)))))