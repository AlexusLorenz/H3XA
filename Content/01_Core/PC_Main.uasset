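; Main player controller that drives game flow between menu, play, highscore entry and highscore states, toggling HUD_Main screens and broadcasting state changes.
; Forwards clicks, new-game calls and, during Play, a looping-timer cursor trace to the pawn through message calls.
; A Counter event decrements Seconds and ends into highscore entry, but its timer setup is disconnected.
; Axis cursor forwarding and graphics benchmark settings are also unwired.
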(event Custom|CursorUpdate
  ;[0 0 0] Cursor Update
  (Utilities|SwitchControllerState
    (:Play
      (Class|IController|CursorUpdate(Message) (Variables|Default|GetPawnRef) (.HitResult (Class|PlayerController|GetHitResultUnderCursorforObjects (Utilities|Array|MakeArray "ObjectTypeQuery7") false))))))

(event Custom|NewGame
  (Class|IController|NewGame(Message) (Variables|Default|GetPawnRef))
  (CallFunction|StartCountdown))

(event Custom|StartCountdown)

(event Custom|Counter
  (bind _output_get (Variables|Default|SetSeconds (- (stale _output_get) 1)))
  (Default|CallOnCounterChanged _output_get)
  (if (<= (Variables|Default|GetSeconds) 0)
    (CallFunction|EndGame)))

(event Custom|EndGame
  (CallFunction|SetControllerState "NewEnumerator2")
  (Utilities|Time|ClearandInvalidateTimerbyHandle (Variables|Default|GetCountdownTimer)))

(event EventBeginPlay
  ;[0 0 0] Prepare Pawnref
  (Variables|Default|SetPawnRef (Pawn|GetControlledPawn))
  ;[0 0 0] Add Score Widget to HUD
  (bind _ashud_main (Utilities|Casting|CastToHUD_Main (HUD|GetHUD)))
  (Variables|Default|SetHUD _ashud_main)
  ;[0 0 0] Cursor Update
  (bind _returnvalue (Utilities|Time|SetTimerbyEvent (delegate Custom|CursorUpdate) 0.01 true))
  (Variables|Default|SetCursorUpdateTimer _returnvalue)
  (CallFunction|PrepareSettings)
  (bind _returnvalue_2 (UserInterface|CreateWidget "/Game/01_Core/UW_Cursor.UW_Cursor_C"))
  (Class|PlayerController|SetMouseCursorWidget "Default" _returnvalue_2))

(event Input|ActionEvents|InputActionClick
  (params (Key :type Key%20Structure :default "None"))
  (bind _pawnref (Variables|Default|GetPawnRef))
  ;[0 0 0] Click Event
  (:Pressed
    (Class|IController|Click(Message) _pawnref true))
  (:Released
    (Class|IController|Click(Message) _pawnref false)))

(event Input|ActionEvents|InputActionMenu
  (params (Key :type Key%20Structure :default "None"))
  (:Pressed
    (CallFunction|SetControllerState "NewEnumerator0")))

(event Input|AxisEvents|InputAxisCursorX
  (params (AxisValue :type Float%20%28single-precision%29))
  ;[0 0 0] Cursor movement. Use Interface for communication.
)

(event Input|AxisEvents|InputAxisCursorY
  (params (AxisValue :type Float%20%28single-precision%29))
  ;[0 0 0] Cursor movement. Use Interface for communication.
)

(event Input|KeyboardEvents|DebugKeyTab
  (params (Key :type Key%20Structure :default "None") (ActionValue :type Input%20Action%20Value%20Structure))
  (:Pressed
    (CallFunction|SetControllerState "NewEnumerator0")))

(fn ConstructionScript)

(fn SetControllerState
  (params (ControllerState :type E_ControllerStates%20Enum :default "NewEnumerator0"))
  (Variables|Default|SetControllerState ControllerState)
  (Utilities|FlowControl|Sequence
    (:then_0
      (switch Utilities|FlowControl|Switch|SwitchonE_ControllerStates (Variables|Default|GetControllerState)
        (:NewEnumerator0
          (Default|ShowMenu (Variables|Default|GetHUD))
          (Default|HideScore (Variables|Default|GetHUD))
          (Default|HideHighscores (Variables|Default|GetHUD)))
        (:NewEnumerator1
          (Default|HideMenu (Variables|Default|GetHUD))
          (Default|ShowScore (Variables|Default|GetHUD))
          (Default|HideHighscores (Variables|Default|GetHUD)))
        (:NewEnumerator2
          (Default|HideMenu (Variables|Default|GetHUD))
          (Default|HideScore (Variables|Default|GetHUD)))
        (:NewEnumerator3
          (Default|HideMenu (Variables|Default|GetHUD))
          (Default|ShowHighscores (Variables|Default|GetHUD))
          (Default|HideScore (Variables|Default|GetHUD)))))
    (:then_1
      (Default|CallOnStateChanged (Variables|Default|GetControllerState)))))

(fn PrepareSettings)